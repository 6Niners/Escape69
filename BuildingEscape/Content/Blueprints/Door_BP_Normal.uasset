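; Door actor that swings open and closed in yaw when DoorRotate sends open or close requests.
; It caches its initial rotation at BeginPlay, then the Rotation timeline adds a yaw offset to it, so the swing is relative to the placed orientation.
; Closing reverses the same timeline, and a timeline event track plays the Doorlock sound at the door's location.
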(event OpenDoorRequest(DoorRotate)
  ;[1 1 1] Door Rotation Animation
  (bind _rotation (Timeline|Rotation Play)
    (:Update
      (Transformation|SetActorRotation (Math|Rotator|CombineRotators (Math|Rotator|MakeRotator 0.0 0.0 _rotation) (Variables|Default|GetInitial_Rotation))))
    (:PlaySound
      (Audio|PlaySoundatLocation "/Game/Audio/door-lock.door-lock" (Transformation|GetActorLocation) "0, 0, 0" 1.0 1.0 0.0 0 0 0))))

(event CloseDoorRequest(DoorRotate)
  ;[1 1 1] Door Rotation Animation
  (bind _rotation (Timeline|Rotation Reverse)
    (:Update
      (Transformation|SetActorRotation (Math|Rotator|CombineRotators (Math|Rotator|MakeRotator 0.0 0.0 _rotation) (Variables|Default|GetInitial_Rotation))))
    (:PlaySound
      (Audio|PlaySoundatLocation "/Game/Audio/door-lock.door-lock" (Transformation|GetActorLocation) "0, 0, 0" 1.0 1.0 0.0 0 0 0))))

(event EventBeginPlay
  ;[1 1 1] Door Rotation Animation
  (Variables|Default|SetInitial_Rotation (Transformation|GetActorRotation)))

(fn ConstructionScript)