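; Room 1 puzzle key actor that the Shinbi player character can trigger with a left mouse click while overlapping it.
; Begin and end overlap enable and disable the actor's input for player controller 0.
; A click sets the Triggered flag and plays a stone snap sound at the location of the actor's Owner; nothing here reads or resets the flag.
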(event Collision|EventActorEndOverlap
  (params (OtherActor :type Actor%20Object%20Reference))
  (Utilities|Casting|CastToShinbiPlayerCharacter OtherActor)
  (Input|DisableInput (Game|GetPlayerController 0)))

(event Collision|EventActorBeginOverlap
  (params (OtherActor :type Actor%20Object%20Reference))
  (Utilities|Casting|CastToShinbiPlayerCharacter OtherActor)
  (Input|EnableInput (Game|GetPlayerController 0)))

(event Input|MouseEvents|LeftMouseButton
  (params (Key :type Key%20Structure :default "None"))
  (:Pressed
    (Variables|Default|SetTriggered true)
    (Audio|PlaySoundatLocation "/Game/Audio/Stone_-_Soundsnap.Stone_-_Soundsnap" (Transformation|GetActorLocation (Components|GetOwner)) "0, 0, 0" 1.0 1.0 0.0 0 0 0)))

(fn ConstructionScript)