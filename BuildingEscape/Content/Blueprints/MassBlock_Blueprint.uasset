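; MassBlock is an actor that shows a mass label when the player pawn is nearby.
; The construction script writes MassVal into the MassText component.
; Every Tick, it measures the distance to the player pawn, shows MassText and Glass within 200 units and hides them otherwise.
; While visible, MassText turns to face the player through a look-at rotation taken from the actor's location.
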(event EventTick
  (params (DeltaSeconds :type Float%20%28single-precision%29))
  (bind _returnvalue (Game|Player|GetPlayerPawn 0))
  (bind _returnvalue_2 (Transformation|GetActorLocation))
  (bind _mass_text (Variables|Default|GetMass_Text))
  (bind _returnvalue_3 (Transformation|GetActorLocation _returnvalue))
  (if (< (Math|Vector|VectorLength (- _returnvalue_3 _returnvalue_2)) 2e+02)
    (Rendering|SetVisibility _mass_text true false)
    (Transformation|SetWorldRotation _mass_text (Math|Rotator|FindLookatRotation _returnvalue_2 _returnvalue_3) false false)
    (else
      (Rendering|SetVisibility _mass_text false false))))

(fn ConstructionScript
  (Rendering|Components|TextRender|SetText (Variables|Default|GetMass_Text) (Variables|Default|GetMass_Val)))