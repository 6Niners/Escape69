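; KnapSackItem is a replicated item with a configurable mass and price, shown as floating KG and $ text labels.
; On BeginPlay, the authority enables replication, overrides the mesh mass and passes the value to the Price1 component.
; The construction script builds label text from MassVal and PriceVal.
; Tick shows the labels only when player pawn 0 is nearby and rotates them to face that pawn.
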(event EventBeginPlay
  (Networking|SwitchHasAuthority
    (:Authority
      (Class|Actor|SetReplicateMovement (Math|Conversions|ToBoolean(Integer) 1))
      (Networking|SetReplicates (Math|Conversions|ToBoolean(Integer) 1))
      (Class|PrimitiveComponent|SetMassOverrideinKg (Variables|Debug|GetStaticMeshComponent) "None" (Math|Conversions|ToFloat(Integer) (Variables|Default|GetMass_Val)) true)
      (Class|Price|SetPrice (Variables|Default|Getprice1) (Variables|Default|GetPrice_Val)))))

(event EventTick
  (params (DeltaSeconds :type Float%20%28single-precision%29))
  (bind _returnvalue (Game|Player|GetPlayerPawn 0))
  (bind _returnvalue_2 (Transformation|GetActorLocation))
  (bind _mass_text (Variables|Default|GetMass_Text))
  (bind _returnvalue_3 (Transformation|GetActorLocation _returnvalue))
  (if (< (Math|Vector|VectorLength (- _returnvalue_3 _returnvalue_2)) 3e+02)
    (Rendering|SetVisibility _mass_text true false)
    (Transformation|SetWorldRotation _mass_text (Math|Rotator|FindLookatRotation _returnvalue_2 _returnvalue_3) false false)
    (else
      (Rendering|SetVisibility _mass_text false false))))

(fn ConstructionScript
  (Rendering|Components|TextRender|SetText (Variables|Default|GetMass_Text) (Utilities|Text|ToText(String) (Utilities|String|Append (Utilities|String|ToString(Integer) (Variables|Default|GetMass_Val)) "KG")))
  (Rendering|Components|TextRender|SetText (Variables|Default|GetPrice_Text) (Utilities|Text|ToText(String) (Utilities|String|Append (Utilities|String|ToString(Integer) (Variables|Default|GetPrice_Val)) "$"))))